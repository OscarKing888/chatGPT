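; BP_MonsterCharacter is a monster character that spots pawns with PawnSensing and marks them as attack targets.
; When it sees a pawn, it writes that pawn into the AttackTarget key of its controller's Blackboard, for AI logic to use.
; Every tick it draws a debug cone along the controller's desired rotation, sized by the sight radius and peripheral vision angle.
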(event OnSeePawn(PawnSensing)
  (params (Pawn :type Pawn%20Object%20Reference))
  (AI|Components|Blackboard|SetValueasObject (AI|GetBlackboard (Pawn|GetController)) (Utilities|Name|MakeLiteralName "AttackTarget") Pawn))

(event EventBeginPlay)

(event Collision|EventActorBeginOverlap
  (params (OtherActor :type Actor%20Object%20Reference)))

(event EventTick
  (params (DeltaSeconds :type Float%20%28single-precision%29))
  (bind _pawnsensing (Variables|Default|GetPawnSensing))
  (bind _returnvalue (Class|PawnSensingComponent|GetPeripheralVisionAngle _pawnsensing))
  (Class|KismetSystemLibrary|DrawDebugConeinDegrees (Transformation|GetActorLocation) (Math|Rotator|GetRotationXVector (Pawn|GetDesiredRotation (Pawn|GetController))) (Variables|/Script/AIModule.PawnSensingComponent|GetSightRadius _pawnsensing) _returnvalue _returnvalue 12 "(R=1.000000,G=1.000000,B=1.000000,A=1.000000)" 0.0 0.0))

(fn ConstructionScript)